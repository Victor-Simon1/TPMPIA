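; BP_MyCharacter is the player character, handling movement, ingot collection and the on-screen interface.
; Axis inputs move it along its yaw-only forward and right vectors and turn it through controller yaw.
; It creates WBP_Interface on begin play, sends it the guard tracking state every tick and updates its ingot count through GetIngot.
; An overlap runs a 90-degree SeeActor check, but the result triggers nothing.
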(event `self.ReceiveBeginPlay`
  (bind _returnvalue (`|CreateWidget` "/Game/Blueprint/WBP_Interface.WBP_Interface_C"))
  (bind _output_get (set `self.UI` _returnvalue))
  (`UserWidget.AddToViewport` _output_get 0))

(event `self.ReceiveTick`
  (params (DeltaSeconds :type "Float (single-precision)"))
  (`/Game/Blueprint/WBP_Interface.GuardTracking` (`self.UI`) (`self.IsTracking`)))

(event `InputAxis|MoveForward`
  (params (AxisValue :type "Float (single-precision)"))
  ;[1 1 1] Movement Forward
  (`self.AddMovementInput` (`KismetMathLibrary.GetForwardVector` (`KismetMathLibrary.MakeRotator` 0.0 0.0 (.yaw (`self.K2_GetActorRotation`)))) AxisValue))

(event `InputAxis|Right`
  (params (AxisValue :type "Float (single-precision)"))
  ;[1 1 1] Movement Right
  (`self.AddMovementInput` (`KismetMathLibrary.GetRightVector` (`KismetMathLibrary.MakeRotator` 0.0 0.0 (.yaw (`self.K2_GetActorRotation`)))) AxisValue))

(event `InputAxis|Turn`
  (params (AxisValue :type "Float (single-precision)"))
  (`self.AddControllerYawInput` AxisValue)
  (`self.K2_SetActorRotation` (`self.K2_GetActorRotation`)))

(event `self.ReceiveActorBeginOverlap`
  (params (OtherActor :type "Actor Object Reference"))
  (`|ExecutionSequence`
    (:`then_0`
      (bind _seeactor (`/Game/Blueprint/Character/SeeObject.SeeActor` self OtherActor))
      (if _seeactor
        _))))

(event `GetIngot`
  (bind _output_get (set `self.Nb_Ingot` (+ (`self.Nb_Ingot`) 1)))
  (`/Game/Blueprint/WBP_Interface.GetIngot` (`self.UI`) _output_get))

(fn `UserConstructionScript`)