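; BP_Guard is a guard actor that slides along world X each tick and changes its cube's color on overlap.
; Movement is a fixed, unswept per-frame offset, not scaled by delta time.
; Overlap begin and end pass red and green to GoToPlayer, which only recolors through a dynamic material instance.
; The recolor requires the other actor's display name to match player controller 0's, not the pawn's.
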(event `self.ReceiveTick`
  (params (DeltaSeconds :type "Float (single-precision)"))
  (`self.K2_SetActorLocation` (+ (`self.K2_GetActorLocation`) (1.0 0.0 0.0))))

(event `self.ReceiveActorBeginOverlap`
  (params (OtherActor :type "Actor Object Reference"))
  (`self.GoToPlayer` OtherActor (`self.Red`)))

(event `self.ReceiveActorEndOverlap`
  (params (OtherActor :type "Actor Object Reference"))
  (`self.GoToPlayer` OtherActor (`self.Green`)))

(fn `GoToPlayer`
  (params (Actor :type "Actor Object Reference") (Color :type "LinearColor Structure"))
  (if (`KismetStringLibrary.EqualEqual_StrStr` (`KismetSystemLibrary.GetDisplayName` Actor) (`KismetSystemLibrary.GetDisplayName` (`GameplayStatics.GetPlayerController` 0)))
    (bind _returnvalue (`PrimitiveComponent.CreateDynamicMaterialInstance` (`self.Cube`) 0 null "None"))
    (`MaterialInstanceDynamic.SetVectorParameterValue` _returnvalue "Color" Color)))

(fn `UserConstructionScript`)