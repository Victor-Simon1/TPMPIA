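; BP_Door is a door actor that swings open when the top-down player character enters its trigger box.
; The BoxCollide overlap casts to BP_TopDownCharacter and plays the DoorTimer timeline, whose track drives the door mesh's relative yaw toward -90 degrees.
; No logic here closes the door again.
; The construction script creates a dynamic material instance on the door frame and gives it a random color.
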(event `self.ReceiveBeginPlay`)

(event `self.BoxCollide.OnComponentBeginOverlap`
  (params (OverlappedComponent :type "PrimitiveComponent Object Reference") (OtherActor :type "Actor Object Reference") (OtherComp :type "PrimitiveComponent Object Reference") (OtherBodyIndex :type Integer) (bFromSweep :type Boolean) (SweepResult :type "HitResult Structure (by ref)"))
  (cast `/Game/TopDown/Blueprints/BP_TopDownCharacter` OtherActor)
  (bind (_direction _newtrack_0) (`Timeline|DoorTimer`)
    (:`Update`
      (`SceneComponent.K2_SetRelativeRotation` (`self.SM_Door`) (`KismetMathLibrary.MakeRotator` 0.0 0.0 (* _newtrack_0 -90.0)) false false))))

(fn `UserConstructionScript`
  (bind _returnvalue (`PrimitiveComponent.CreateDynamicMaterialInstance` (`self.SM_DoorFrame`) 0 null "None"))
  (`MaterialInstanceDynamic.SetVectorParameterValue` _returnvalue "Color" (`KismetMathLibrary.MakeColor` (`KismetMathLibrary.RandomFloatInRange` 0.0 1.0) (`KismetMathLibrary.RandomFloatInRange` 0.0 1.0) (`KismetMathLibrary.RandomFloatInRange` 0.0 1.0))))